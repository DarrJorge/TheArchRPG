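; Base hit react gameplay ability, activated by event, that plays an enemy's reaction to being hit.
; It optionally rotates the enemy toward the event instigator, then plays a random hit react montage, or waits briefly if none is set, before ending.
; A material scalar parameter highlights the mesh until the ability ends.
; Activation also applies the GE_DamageTaken effect to the owner.
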(event Ability|EventOnEndAbility
  (params (bWasCancelled :type Boolean))
  (CallFunction|SetHighlightHitActor 0.0))

(event Ability|EventActivateAbilityFromEvent
  (params (EventData :type Gameplay%20Event%20Data%20Structure%20%28by%20ref%29))
  (Utilities|FlowControl|Sequence
    (:then_0
      (if (Variables|Default|GetFaceAttacker)
        (CallFunction|RotateHitActortoInstigator (Variables|Default|GetCurrentEventData))))
    (:then_1
      (if (Variables|Default|GetHasHitReactMontage)
        (|PlayMontageandWaitProxy "None" (.OutItem (Utilities|Array|Random (Variables|Default|GetHitReactAnimMontages))) 1.0 "None" true 1.0 0.0 false
          (:then
            (CallFunction|SetHighlightHitActor 1.0))
          (:OnCompleted
            (Ability|EndAbility :!label _label))
          (:OnBlendOut
            (goto _label))
          (:OnInterrupted
            (goto _label))
          (:OnCancelled
            (goto _label)))
        (else
          (CallFunction|SetHighlightHitActor 1.0)
          (if (not (Variables|Default|GetHasHitReactMontage))
            (Utilities|FlowControl|Delay 0.2)
            (Ability|EndAbility)))))
    (:then_2
      (Ability|ApplyGameplayEffectSpecToOwner (Ability|MakeOutgoingGameplayEffectSpec "/Game/ArchAll/AbilitySystem/Shared/GameplayEffects/GE_DamageTaken.GE_DamageTaken_C")))))

(fn RotateHitActortoInstigator
  (params (GameplayEventData :type Gameplay%20Event%20Data%20Structure%20%28by%20ref%29))
  (Transformation|SetActorRotation (Class|ArchEnemyGameplayAbility|GetEnemyCharacterfromActorInfo) (Math|Rotator|FindLookatRotation (Transformation|GetActorLocation (Class|ArchEnemyGameplayAbility|GetEnemyCharacterfromActorInfo)) (Transformation|GetActorLocation (.Instigator (Utilities|Struct|BreakGameplayEventData GameplayEventData))))))

(fn SetHighlightHitActor
  (params (HighlightValue :type Float%20%28double-precision%29))
  (Rendering|Material|SetScalarParameterValueonMaterials (Class|GameplayAbility|GetOwningComponentfromActorInfo) "HitFxSwitch" HighlightValue))