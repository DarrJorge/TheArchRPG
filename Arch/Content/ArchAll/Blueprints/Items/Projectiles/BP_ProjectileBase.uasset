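; BP_ProjectileBase is a base projectile Blueprint that handles the sound and visual effects of a projectile's spawn, flight and impact.
; BeginPlay plays the spawn sound, attaches a flying sound that stops with the projectile, and spawns a forward-facing muzzle effect.
; OnSpawnProjectileHitFX plays impact sound and effect at the hit location, with the effect spawning only when the hit sound is valid.
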(event EventBeginPlay
  (CallFunction|PlaySoundSpawnProjectile)
  (CallFunction|PlaySoundFlyingProjectile)
  (CallFunction|PlayMuzzleFX))

(event EventOnSpawnProjectileHitFX
  (params (HitLocation :type Vector%20%28by%20ref%29 :default "0, 0, 0"))
  (bind _projectilehitsound (Variables|Default|GetProjectileHitSound)
    (:then
      (Audio|PlaySoundatLocation _projectilehitsound HitLocation "0, 0, 0" 1.0 1.0 0.0 0 0 0 0)
      (bind _projectilehitfx (Variables|Default|GetProjectileHitFX)
        (:then
          (Niagara|SpawnSystematLocation _projectilehitfx HitLocation))
        (:else)))
    (:else)))

(fn ConstructionScript)

(fn PlaySoundSpawnProjectile
  (bind _projectilespawnsound (Variables|Default|GetProjectileSpawnSound)
    (:then
      (Audio|PlaySoundatLocation _projectilespawnsound (Transformation|GetActorLocation) "0, 0, 0" 1.0 1.0 0.0 0 0 0 0))
    (:else)))

(fn PlaySoundFlyingProjectile
  (bind _projectileflyingsound (Variables|Default|GetProjectileFlyingSound)
    (:then
      (Audio|SpawnSoundAttached _projectileflyingsound (Variables|Transformation|GetRootComponent) "None" "0, 0, 0" "0, 0, 0" "KeepRelativeOffset" true 1.0 1.0 0.0 0 0))
    (:else)))

(fn PlayMuzzleFX
  (bind _projectilemuzzlefx (Variables|Default|GetProjectileMuzzleFX)
    (:then
      (Niagara|SpawnSystematLocation _projectilemuzzlefx (Transformation|GetActorLocation) (Math|Conversions|RotationFromXVector (Transformation|GetActorForwardVector))))
    (:else)))